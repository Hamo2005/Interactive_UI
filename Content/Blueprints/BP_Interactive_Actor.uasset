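; Interactive actor base that shows a UI widget when a Character enters its sphere.
; Other overlaps and every exit run a sphere trace at the same radius to decide whether any Character keeps it visible, with debug drawing and printing left on.
; The WB_Interactive_UI widget is created lazily on overlap events, and InteractiveUIData is pushed into it on later overlaps and through its OnRep.
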(event `self.Sphere.OnComponentBeginOverlap`
  (params (OverlappedComponent :type "PrimitiveComponent Object Reference") (OtherActor :type "Actor Object Reference") (OtherComp :type "PrimitiveComponent Object Reference") (OtherBodyIndex :type Integer) (bFromSweep :type Boolean) (SweepResult :type "HitResult Structure (by ref)"))
  (bind _widget_root (`self.Widget Root`))
  (bind _widget_root_2 (`self.Widget Root`))
  ;[1 1 1] Update
  (cast `Character` OtherActor
    (:`then`
      (`SceneComponent.SetVisibility` _widget_root_2 true false))
    (:`CastFailed`
      (bind _found_players (`self.Check For Player Around` :!label _label))
      (`SceneComponent.SetVisibility` _widget_root_2 _found_players false)))
  (`/Engine/EditorBlueprintResources/StandardMacros.IsValid` (`WidgetComponent.GetWidget` _widget_root)
    (:`Is Valid`
      (`self.Update Widget Data`))
    (:`Is Not Valid`
      (bind _returnvalue (`|CreateWidget` "/Game/Blueprints/UI/Interactive/WB_Interactive_UI.WB_Interactive_UI_C" null (`self.Interactive UI Data`)))
      (`WidgetComponent.SetWidget` _widget_root _returnvalue))))

(event `self.Sphere.OnComponentEndOverlap`
  (params (OverlappedComponent :type "PrimitiveComponent Object Reference") (OtherActor :type "Actor Object Reference") (OtherComp :type "PrimitiveComponent Object Reference") (OtherBodyIndex :type Integer))
  ;[1 1 1] Update
  (goto _label))

(event `Update Widget Data`
  (bind _returnvalue (`WidgetComponent.GetWidget` (`self.Widget Root`)))
  ;[1 1 1] Update Widget Data
  (`/Engine/EditorBlueprintResources/StandardMacros.IsValid` _returnvalue
    (:`Is Valid`
      (bind _aswb_interactive_ui (cast `/Game/Blueprints/UI/Interactive/WB_Interactive_UI` _returnvalue))
      (set `/Game/Blueprints/UI/Interactive/WB_Interactive_UI.Interactive UI Data` (`self.Interactive UI Data`) _aswb_interactive_ui))))

(fn `Check For Player Around`
  (returns (`Found Players` :type Boolean))
  (locals (Players :type "Array of Character Object Reference"))
  (bind _sphere (`self.Sphere`))
  (bind _returnvalue (`SceneComponent.K2_GetComponentLocation` _sphere))
  ;[1 1 1] Check For Player Around
  (`KismetArrayLibrary.Array_Clear` (`local.Players`))
  (bind _outhits (`KismetSystemLibrary.SphereTraceMulti` :`Start` _returnvalue :`End` _returnvalue :`Radius` (`SphereComponent.SphereRadius` _sphere) :`TraceChannel` "TraceTypeQuery1" :`bTraceComplex` true :`DrawDebugType` "ForDuration"))
  (for _array_element _outhits
    (bind _ascharacter (cast `Character` (`.HitActor` (`GameplayStatics.BreakHitResult` _array_element))))
    (`KismetArrayLibrary.Array_Add` (`local.Players`) _ascharacter)
    (`KismetSystemLibrary.PrintString` "Hello"))
  (return (not (`KismetArrayLibrary.Array_IsEmpty` (`local.Players`)))))

(fn `OnRep_Interactive UI Data`
  (`self.Update Widget Data`))

(fn `UserConstructionScript`)